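; Interactable door that swings open or closed, set up to require several taps per interaction.
; Interact toggles IsOpen, plays a sound at the door and runs OpenDoorTimeline forward or in reverse to drive the mesh's yaw.
; Getter functions supply the interaction type, location, tap count, zero hold duration and an open/close prompt that follows IsOpen.
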(event Custom|CloseDoor
  (Variables|Default|SetisOpen? false)
  (Audio|PlaySoundatLocation "/Engine/VREditor/Sounds/UI/Leave_Simulate.Leave_Simulate" (Transformation|GetActorLocation) "0, 0, 0" 1.0 1.0 0.0 0 0 0 0)
  (bind _zrotation (Timeline|OpenDoorTimeline Reverse)
    (:Update
      (Transformation|SetRelativeRotation (Variables|Default|GetDoorMesh) (Math|Rotator|MakeRotator 0.0 0.0 _zrotation) false false))))

(event Custom|OpenDoor
  (Variables|Default|SetisOpen? true)
  (Audio|PlaySoundatLocation "/Engine/VREditor/Sounds/UI/Enter_Play.Enter_Play" (Transformation|GetActorLocation) "0, 0, 0" 1.0 1.0 0.0 0 0 0 0)
  (bind _zrotation (Timeline|OpenDoorTimeline Play)
    (:Update
      (Transformation|SetRelativeRotation (Variables|Default|GetDoorMesh) (Math|Rotator|MakeRotator 0.0 0.0 _zrotation) false false))))

(event EventInteract
  (params (Interactor :type Actor%20Object%20Reference))
  (if (Variables|Default|GetisOpen?)
    (CallFunction|CloseDoor)
    (else
      (CallFunction|OpenDoor))))

(fn ConstructionScript)

(fn GetHoldDuration
  (return 0.0))

(fn GetInteractionLocation
  (return (Transformation|GetWorldLocation (Variables|Default|GetInteractionLocation))))

(fn GetInteractionPrompt
  (return (Utilities|String|SelectText "to close the door" "to open the door" (Variables|Default|GetisOpen?))))

(fn GetInteractionType
  (return (Variables|Default|GetInteractionType)))

(fn GetTapCount
  (return 4) ; door needs to be tapped (tap count) times
)