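; BP_NPC is an interactable character that offers a "to talk" prompt to whoever interacts with it.
; On Interact it snaps its yaw to face the interactor and plays a ping sound at its own location as a greeting.
; Getter functions describe the interaction: fixed prompt, type, zero hold time and tap count, plus a world position taken from its InteractionLocation component.
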(event EventBeginPlay)

(event Collision|EventActorBeginOverlap
  (params (OtherActor :type Actor%20Object%20Reference)))

(event EventTick
  (params (DeltaSeconds :type Float%20%28single-precision%29)))

(event EventInteract
  (params (Interactor :type Actor%20Object%20Reference))
  (Transformation|SetActorRotation (Math|Rotator|MakeRotator 0.0 0.0 (.yaw (Math|Rotator|FindLookatRotation (Transformation|GetActorLocation) (Transformation|GetActorLocation Interactor))))) ; turn npc to look at player
  (Audio|PlaySoundatLocation "/Engine/EngineSounds/1kSineTonePing.1kSineTonePing" (Transformation|GetActorLocation) "0, 0, 0" 1.0 1.0 0.0 0 0 0 0) ; say hi
)

(fn ConstructionScript)

(fn GetHoldDuration
  (return 0.0))

(fn GetInteractionLocation
  (return (Transformation|GetWorldLocation (Variables|Default|GetInteractionLocation))))

(fn GetInteractionPrompt
  (return "to talk"))

(fn GetInteractionType
  (return "NewEnumerator0"))

(fn GetTapCount
  (return 0))