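; BP_Typewriter is an interactable save point that stores the player's progress.
; On Interact it casts the interactor to BP_FirstPersonCharacter, passes GetPlayerSave to the GameInstance's async SavePlayerMessage, and plays a confirmation tone.
; BeginPlay briefly disables the Sphere's collision as a workaround for the player overlapping it immediately on game load.
; Interaction getters expose InteractionType and otherwise return empty or zero values.
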(event EventBeginPlay
  ;[1 1 1] an absolutely hideous fix. very amateurish. lets the thing load because you're immediately overlapping with its collision sphere upon game loading at the start.
  (Collision|SetCollisionEnabled (Variables|Default|GetSphere) "NoCollision")
  (Utilities|FlowControl|Delay 0.2)
  (Collision|SetCollisionEnabled (Variables|Default|GetSphere) "QueryOnly"))

(event EventInteract
  (params (Interactor :type Actor%20Object%20Reference))
  (bind _asbp_first_person_character (Utilities|Casting|CastToBP_FirstPersonCharacter Interactor)) ; if this is true, the player has reached a checkpoint
  (bind _playersave (Default|GetPlayerSave _asbp_first_person_character)) ; the first person character has the information we want to save
  (Class|BPISaveGame|SavePlayer(Message) (Game|GetGameInstance) _playersave true)
  (Audio|PlaySound2D "/Engine/EngineSounds/1kSineTonePing.1kSineTonePing" 1.0 1.0 0.0 0 0) ; plays a sound to indicate game saved
)

(fn ConstructionScript)

(fn GetHoldDuration
  (return 0.0))

(fn GetInteractionLocation
  (return "0, 0, 0"))

(fn GetInteractionPrompt
  (return ""))

(fn GetInteractionType
  (return (Variables|Default|GetInteractionType)))

(fn GetTapCount
  (return 0))