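; BPC_Inventory is an inventory component that stores items with quantities in an array.
; Its AddItem event adds each item and quantity pair with AddUnique, so only identical pairs are deduplicated and quantities never stack.
; Debug strings report startup, the added item's class name and the class name of the array's first entry, which is not necessarily the new item.
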(event EventBeginPlay
  (Development|PrintString "BPC_INVENTORY up and running"))

(event EventTick
  (params (DeltaSeconds :type Float%20%28single-precision%29)))

(event EventAddItem
  (params (Item :type BP%20Inventory%20Item%20Class%20Reference) (Quantity :type Integer))
  (bind _itemarray (Variables|Default|GetItemArray))
  (Utilities|Array|AddUnique _itemarray (Utilities|Struct|MakeS_InventoryItems Item Quantity))
  (Development|PrintString (Utilities|GetClassDisplayName Item))
  (Development|PrintString (Utilities|String|Append (Utilities|GetClassDisplayName (.Item (Utilities|Struct|BreakS_InventoryItems (Utilities|Array|Get(acopy) _itemarray)))) " found in the array")))